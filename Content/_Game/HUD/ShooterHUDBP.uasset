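; Shooter HUD that draws a dynamic four-part crosshair slightly above screen center.
; BeginPlay caches the player's ShooterCharacterBP, and DrawHUD re-acquires it if the reference is invalid.
; Each frame it reads the character's spread multiplier and pushes the top, bottom, left and right textures outward by that times the max spread.
; Texture half-size is subtracted from the anchor to keep the crosshair centered.
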(event `self.ReceiveBeginPlay`
  ;[1 1 1] Get ShooterCharacter REF
  (if (not (`KismetSystemLibrary.IsValid` (`self.ShooterCharacter`)))
    (bind _asshooter_character_bp (cast `/Game/_Game/Character/ShooterCharacterBP` (`GameplayStatics.GetPlayerPawn` 0)))
    (set `self.ShooterCharacter` _asshooter_character_bp)))

(event `self.ReceiveDrawHUD`
  (params (SizeX :type Integer) (SizeY :type Integer))
  (bind (_x _y) (`KismetMathLibrary.BreakVector2D` (`self.CenterScreen`)))
  (bind (_x_2 _y_2) (`KismetMathLibrary.BreakVector2D` (`self.CrosshairBaseCenter`)))
  (bind (_x_3 _y_3) (`KismetMathLibrary.BreakVector2D` (`self.CrosshairBaseCenter`)))
  (bind (_x_4 _y_4) (`KismetMathLibrary.BreakVector2D` (`self.CrosshairBaseCenter`)))
  (bind (_x_5 _y_5) (`KismetMathLibrary.BreakVector2D` (`self.CrosshairBaseCenter`)))
  (bind (_x_6 _y_6) (`KismetMathLibrary.BreakVector2D` (`self.CrosshairLocation`)))
  ;[1 1 1] Ekranın boyutunu da verir. Event Tick gibi çalışır.
  (set `self.CenterScreen` (`KismetMathLibrary.MakeVector2D` (`KismetMathLibrary.Conv_IntToDouble` (/ SizeX 2)) (`KismetMathLibrary.Conv_IntToDouble` (/ SizeY 2))))
  (set `self.CrosshairLocation` (`KismetMathLibrary.MakeVector2D` _x (- _y 50.0)))
  ;;[1 1 1] Shooter karakter geçerli mi
  (if (not (`KismetSystemLibrary.IsValid` (`self.ShooterCharacter`)))
    (bind _asshooter_character_bp (cast `/Game/_Game/Character/ShooterCharacterBP` (`GameplayStatics.GetPlayerPawn` 0)))
    (bind _output_get (set `self.ShooterCharacter` _asshooter_character_bp)))
  (set `self.CrosshairSpreadMultiplier` (`ShooterCharacter.GetCrosshairSpreadMultiplier` _output_get))
  ;[1 1 1] Ekran ortası
  (set `self.CrosshairBaseCenter` (`KismetMathLibrary.MakeVector2D` (- _x_6 (`self.CrosshairHalfWidth`)) (- _y_6 (`self.CrosshairHalfHeight`))))
  (`self.DrawTexture` "/Game/Assets/Textures/Crosshairs/Crosshair_Quad_9_Bottom.Crosshair_Quad_9_Bottom" _x_4 (+ _y_4 (* (`self.CrosshairSpreadMax`) (`self.CrosshairSpreadMultiplier`))) 64.0 64.0 0.0 0.0 1.0 1.0 :!pinned true) ; Screen W ve Screen H : Texture boyutu\nUWidth ve VHeight: Ekrana ne oranda yerleştirileceği. 1 e 1 dersek tek bir tane çizilir.\nBurada dikkat edilmesi gereken ekran ortası dediğimizde texture bıyutunu düşmemiz gerekiyor\nYoksa texture boyutu kadar kayma yaşanır.
  (`self.DrawTexture` "/Game/Assets/Textures/Crosshairs/Crosshair_Quad_9_Top.Crosshair_Quad_9_Top" _x_5 (- _y_5 (* (`self.CrosshairSpreadMax`) (`self.CrosshairSpreadMultiplier`))) 64.0 64.0 0.0 0.0 1.0 1.0 :!pinned true) ; Screen W ve Screen H : Texture boyutu\nUWidth ve VHeight: Ekrana ne oranda yerleştirileceği. 1 e 1 dersek tek bir tane çizilir.\nBurada dikkat edilmesi gereken ekran ortası dediğimizde texture bıyutunu düşmemiz gerekiyor\nYoksa texture boyutu kadar kayma yaşanır.
  (`self.DrawTexture` "/Game/Assets/Textures/Crosshairs/Crosshair_Quad_9_Left.Crosshair_Quad_9_Left" (- _x_3 (* (`self.CrosshairSpreadMax`) (`self.CrosshairSpreadMultiplier`))) _y_3 64.0 64.0 0.0 0.0 1.0 1.0 :!pinned true) ; Screen W ve Screen H : Texture boyutu\nUWidth ve VHeight: Ekrana ne oranda yerleştirileceği. 1 e 1 dersek tek bir tane çizilir.\nBurada dikkat edilmesi gereken ekran ortası dediğimizde texture bıyutunu düşmemiz gerekiyor\nYoksa texture boyutu kadar kayma yaşanır.
  (`self.DrawTexture` "/Game/Assets/Textures/Crosshairs/Crosshair_Quad_9_Right.Crosshair_Quad_9_Right" (+ _x_2 (* (`self.CrosshairSpreadMax`) (`self.CrosshairSpreadMultiplier`))) _y_2 64.0 64.0 0.0 0.0 1.0 1.0 :!pinned true) ; Screen W ve Screen H : Texture boyutu\nUWidth ve VHeight: Ekrana ne oranda yerleştirileceği. 1 e 1 dersek tek bir tane çizilir.\nBurada dikkat edilmesi gereken ekran ortası dediğimizde texture bıyutunu düşmemiz gerekiyor\nYoksa texture boyutu kadar kayma yaşanır.
)

(fn `UserConstructionScript`)